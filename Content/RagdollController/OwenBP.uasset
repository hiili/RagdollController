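; OwenBP is a test Blueprint that drives one motor of a ragdoll's joints from player input.
; Each Tick scales the Turn and LookUp axes into a large motor command for a single hard-coded joint, then prints that joint's angles and command.
; SetJointMotorCommand copies, edits and writes back the JointState array element, working around an engine issue with setting struct members inside arrays.
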(event EventTick
  (params (DeltaSeconds :type Float%20%28single-precision%29))
  (bind _jointstates (Variables|Default|GetJointStates))
  (bind _item (Utilities|Array|Get(acopy) _jointstates 8))
  (bind (_jointangles _motorcommand) (Utilities|Struct|BreakJointState _item))
  (CallFunction|SetJointMotorCommand (Variables|Default|GetJointStates) 8 (* (Math|Vector|MakeVector (Input|AxisValues|GetTurn) (Input|AxisValues|GetLookUp) 0.0) 1e+05))
  (Development|PrintString (Utilities|String|BuildString(Vector) (Utilities|String|BuildString(Vector) "" "Angles: " _jointangles) " Motor: " _motorcommand)))

(event EventBeginPlay
  (Input|EnableInput (Game|GetPlayerController 0)))

(fn ConstructionScript)

(fn SetJointMotorCommand
  (params (JointState%20Array :type Array%20of%20Joint%20State%20Structures) (Joint%20Index :type Integer) (Motor%20Command :type Vector :default "0, 0, 0"))
  ;[1 1 1] Set the Motor Command element of a single joint in a JointState array (workaround for http://answers.unrealengine.com/questions/91479/)
  (LocalVariables|SetTemporary%20JointState (Utilities|Array|Get(acopy) JointState%20Array Joint%20Index))
  (Utilities|Struct|SetmembersinJointState (LocalVariables|GetTemporary%20JointState) Motor%20Command)
  (Utilities|Array|SetArrayElem JointState%20Array Joint%20Index (LocalVariables|GetTemporary%20JointState)))